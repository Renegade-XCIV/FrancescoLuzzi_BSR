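; One-way door actor that the player swings open with E, until a lock trigger disables it.
; Overlapping CloseToDoor opens a Tick gate that polls the key and plays a yaw timeline; leaving closes the gate and reverses it.
; Any overlap with three KeepDoorLocked volumes clears DoorCanBeOpened and turns the lamp red, with no re-enable here.
; It creates its own WB_PlayerUI widget for text.
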(event OnComponentBeginOverlap(CloseToDoor)
  (params (OverlappedComponent :type Primitive%20Component%20Object%20Reference) (OtherActor :type Actor%20Object%20Reference) (OtherComp :type Primitive%20Component%20Object%20Reference) (OtherBodyIndex :type Integer) (bFromSweep :type Boolean) (SweepResult :type Hit%20Result%20Structure%20%28by%20ref%29))
  (if (== OtherActor (Game|Player|GetPlayerPawn 0))
    (Utilities|FlowControl|Gate true) ; enters at Open
  ))

(event OnComponentEndOverlap(CloseToDoor)
  (params (OverlappedComponent :type Primitive%20Component%20Object%20Reference) (OtherActor :type Actor%20Object%20Reference) (OtherComp :type Primitive%20Component%20Object%20Reference) (OtherBodyIndex :type Integer))
  (if (== OtherActor (Game|Player|GetPlayerPawn 0))
    (Utilities|FlowControl|Sequence
      (:then_0
        (Utilities|FlowControl|Gate true) ; enters at Close
      )
      (:then_1
        (Variables|/Script/UMG.TextBlock|SetText (Variables|/Game/Blueprints/WB_PlayerUI.WB_PlayerUI_C|GetUIText (Variables|Default|GetTextEmitter)) "")
        (bind _newtrack_0 (Timeline|DoorMovement Reverse)
          (:Update
            (Transformation|SetRelativeRotation (Variables|Default|GetDoor) (Math|Rotator|MakeRotator 0.0 0.0 (Math|Float|Lerp 0.0 9e+01 _newtrack_0)) false false)))))))

(event OnComponentBeginOverlap(KeepDoorLocked)
  (params (OverlappedComponent :type Primitive%20Component%20Object%20Reference) (OtherActor :type Actor%20Object%20Reference) (OtherComp :type Primitive%20Component%20Object%20Reference) (OtherBodyIndex :type Integer) (bFromSweep :type Boolean) (SweepResult :type Hit%20Result%20Structure%20%28by%20ref%29))
  (Variables|Default|SetDoorCanBeOpened false)
  (Rendering|Material|SetMaterial (Variables|Default|GetLamp) 0 "/Game/Materials/M_RedLight.M_RedLight"))

(event OnComponentBeginOverlap(KeepDoorLocked1)
  (params (OverlappedComponent :type Primitive%20Component%20Object%20Reference) (OtherActor :type Actor%20Object%20Reference) (OtherComp :type Primitive%20Component%20Object%20Reference) (OtherBodyIndex :type Integer) (bFromSweep :type Boolean) (SweepResult :type Hit%20Result%20Structure%20%28by%20ref%29))
  (Variables|Default|SetDoorCanBeOpened false)
  (Rendering|Material|SetMaterial (Variables|Default|GetLamp) 0 "/Game/Materials/M_RedLight.M_RedLight"))

(event OnComponentBeginOverlap(KeepDoorLocked2)
  (params (OverlappedComponent :type Primitive%20Component%20Object%20Reference) (OtherActor :type Actor%20Object%20Reference) (OtherComp :type Primitive%20Component%20Object%20Reference) (OtherBodyIndex :type Integer) (bFromSweep :type Boolean) (SweepResult :type Hit%20Result%20Structure%20%28by%20ref%29))
  (Variables|Default|SetDoorCanBeOpened false)
  (Rendering|Material|SetMaterial (Variables|Default|GetLamp) 0 "/Game/Materials/M_RedLight.M_RedLight"))

(event EventBeginPlay
  (bind _returnvalue (UserInterface|CreateWidget "/Game/Blueprints/WB_PlayerUI.WB_PlayerUI_C"))
  (bind _output_get (Variables|Default|SetTextEmitter _returnvalue))
  (UserInterface|Viewport|AddtoViewport _output_get 0)
  (Variables|/Script/UMG.TextBlock|SetText (Variables|/Game/Blueprints/WB_PlayerUI.WB_PlayerUI_C|GetUIText _output_get) ""))

(event Collision|EventActorBeginOverlap
  (params (OtherActor :type Actor%20Object%20Reference)))

(event EventTick
  (params (DeltaSeconds :type Float%20%28single-precision%29))
  (Utilities|FlowControl|Gate true
    (:Exit
      (if (Variables|Default|GetDoorCanBeOpened)
        (Variables|/Script/UMG.TextBlock|SetText (Variables|/Game/Blueprints/WB_PlayerUI.WB_PlayerUI_C|GetUIText (Variables|Default|GetTextEmitter)) "")
        (if (Game|Player|IsInputKeyDown (Game|GetPlayerController 0) "E")
          (bind _newtrack_0 (Timeline|DoorMovement Play)
            (:Update
              (Transformation|SetRelativeRotation (Variables|Default|GetDoor) (Math|Rotator|MakeRotator 0.0 0.0 (Math|Float|Lerp 0.0 9e+01 _newtrack_0)) false false))))))))

(fn ConstructionScript)