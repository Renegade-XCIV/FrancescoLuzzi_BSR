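; Switch-operated door that swings open when the player presses E inside its trigger box, then closes again after a configurable delay.
; Box overlap opens a Tick gate that, if DoorCanBeOpened, shows a UI prompt and polls the key.
; Chained timelines, each played from the previous one's Update, rotate switch and door out and, after Timer, back.
; The lamp turns green on opening and red on closing.
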(event OnComponentBeginOverlap(Box)
  (params (OverlappedComponent :type Primitive%20Component%20Object%20Reference) (OtherActor :type Actor%20Object%20Reference) (OtherComp :type Primitive%20Component%20Object%20Reference) (OtherBodyIndex :type Integer) (bFromSweep :type Boolean) (SweepResult :type Hit%20Result%20Structure%20%28by%20ref%29))
  (if (== OtherActor (Game|Player|GetPlayerPawn 0))
    (Utilities|FlowControl|Gate true) ; enters at Open
  ))

(event OnComponentEndOverlap(Box)
  (params (OverlappedComponent :type Primitive%20Component%20Object%20Reference) (OtherActor :type Actor%20Object%20Reference) (OtherComp :type Primitive%20Component%20Object%20Reference) (OtherBodyIndex :type Integer))
  (if (== OtherActor (Game|Player|GetPlayerPawn 0))
    (Utilities|FlowControl|Sequence
      (:then_0
        (Variables|/Script/UMG.TextBlock|SetText (Variables|/Game/Blueprints/WB_PlayerUI.WB_PlayerUI_C|GetUIText (Variables|Default|GetTextEmitter)) ""))
      (:then_1
        (Utilities|FlowControl|Gate true) ; enters at Close
      ))))

(event EventBeginPlay
  (bind _returnvalue (UserInterface|CreateWidget "/Game/Blueprints/WB_PlayerUI.WB_PlayerUI_C"))
  (bind _output_get (Variables|Default|SetTextEmitter _returnvalue))
  (UserInterface|Viewport|AddtoViewport _output_get 0)
  (Variables|/Script/UMG.TextBlock|SetText (Variables|/Game/Blueprints/WB_PlayerUI.WB_PlayerUI_C|GetUIText _output_get) "")
  (Rendering|Material|SetMaterial (Variables|Default|GetLamp) 0 "/Game/Materials/M_RedLight.M_RedLight"))

(event EventTick
  (params (DeltaSeconds :type Float%20%28single-precision%29))
  (Utilities|FlowControl|Gate true
    (:Exit
      (if (Variables|Default|GetDoorCanBeOpened)
        (Variables|/Script/UMG.TextBlock|SetText (Variables|/Game/Blueprints/WB_PlayerUI.WB_PlayerUI_C|GetUIText (Variables|Default|GetTextEmitter)) "Press E to interact")
        (if (Game|Player|IsInputKeyDown (Game|GetPlayerController 0) "E")
          (bind _newtrack_0 (Timeline|SwitchMovement Play)
            (:Update
              (Transformation|SetRelativeRotation (Variables|Default|GetSwitch) (Math|Rotator|MakeRotator 0.0 (Math|Float|Lerp -3e+01 3e+01 _newtrack_0) -9e+01) false false)
              (bind _newtrack_0_2 (Timeline|DoorMovement Play)
                (:Update
                  (Transformation|SetRelativeRotation (Variables|Default|GetDoor) (Math|Rotator|MakeRotator 0.0 0.0 (Math|Float|Lerp 0.0 9e+01 _newtrack_0_2)) false false)
                  (Rendering|Material|SetMaterial (Variables|Default|GetLamp) 0 "/Game/Materials/M_GreenLight.M_GreenLight")
                  (Utilities|FlowControl|Delay (Variables|Default|GetTimer))
                  (bind _newtrack_0_3 (Timeline|Timeline_0 Play)
                    (:Update
                      (Transformation|SetRelativeRotation (Variables|Default|GetSwitch) (Math|Rotator|MakeRotator 0.0 (Math|Float|Lerp 3e+01 -3e+01 _newtrack_0_3) -9e+01) false false)
                      (bind _newtrack_0_4 (Timeline|Timeline Play)
                        (:Update
                          (Transformation|SetRelativeRotation (Variables|Default|GetDoor) (Math|Rotator|MakeRotator 0.0 0.0 (Math|Float|Lerp 9e+01 0.0 _newtrack_0_4)) false false)
                          (Rendering|Material|SetMaterial (Variables|Default|GetLamp) 0 "/Game/Materials/M_RedLight.M_RedLight"))))))))))))))

(fn ConstructionScript)